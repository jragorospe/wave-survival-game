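; BP_Action_BlackHole is the Black Hole action, gating the ability behind a Rage cost.
; CanStart extends the parent check, requiring valid attributes on the instigator and Rage of at least RageCost, and prints a message when Rage is short.
; StartAction runs the parent logic, then subtracts RageCost through ApplyRage.
; The black hole effect itself is not defined in these graphs.
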(event `self.StartAction`
  (params (Instigator :type "Actor Object Reference"))
  (`parent.StartAction` Instigator)
  (bind _returnvalue (`WaveAttributeComponent.GetAttributes` Instigator))
  (`/Engine/EditorBlueprintResources/StandardMacros.IsValid` _returnvalue
    (:`Is Valid`
      (`WaveAttributeComponent.ApplyRage` _returnvalue Instigator (/ (`self.RageCost`) -1.0)))))

(fn `CanStart`
  (params (Instigator :type "Actor Object Reference"))
  (returns (ReturnValue :type Boolean))
  (bind _returnvalue (`parent.CanStart` Instigator))
  (if _returnvalue
    (bind _returnvalue_2 (`WaveAttributeComponent.GetAttributes` Instigator))
    (`/Engine/EditorBlueprintResources/StandardMacros.IsValid` _returnvalue_2
      (:`Is Valid`
        (if (>= (`WaveAttributeComponent.GetRage` _returnvalue_2) (`self.RageCost`))
          (return true)
          (else
            (`KismetSystemLibrary.PrintString` "Not Enough Rage")
            (return false))))
      (:`Is Not Valid`
        (return false)))
    (else
      (return false))))