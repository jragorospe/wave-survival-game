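; Magic projectile Blueprint that adds area splash damage when it explodes.
; Explode runs ApplySplashDamage before calling the parent's Explode.
; Splash damage hits every Character overlapping the explosion sphere, skipping the instigator and the already-damaged actor, with the instigator as damage causer.
; The overlap query lives in Blueprint because the author could not get it working on the native sphere component.
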(event `self.Explode`
  ;[0 0 1 1 14] Would do this in code but I couldn't get my native Sphere Component to get Overlapped Actors for some reason.
  (`self.ApplySplashDamage`)
  (`parent.Explode`))

(fn `ApplySplashDamage`
  (locals (OverlapActor :type "Actor Object Reference"))
  (for _array_element (`PrimitiveComponent.GetOverlappingActors` (`self.Explosion Sphere Component`) "/Script/Engine.Character")
    (set `local.OverlapActor` _array_element)
    (if (and (!= (`self.DamagedActor`) (`local.OverlapActor`)) (!= (`self.Instigator`) (`local.OverlapActor`)))
      (`WaveGameplayFunctionLibrary.ApplyDamage` (`self.Instigator`) (`local.OverlapActor`) (`self.SplashDamage`)))))

(fn `UserConstructionScript`)